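; BP_AI is an overworld enemy for the turn-based RPG that chases pawns it sees and starts a battle on contact.
; PawnSensing drives AI MoveTo toward the seen pawn, while a retriggerable delay sends it back to its spawn location once sightings stop.
; Overlapping BP_ThirdPersonCharacter starts BattleScene with that pawn, and the AI destroys itself when the battle's end event fires.
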(event OnSeePawn(PawnSensing)
  (params (Pawn :type Pawn%20Object%20Reference))
  (Utilities|FlowControl|Sequence
    (:then_0
      (AI|AIMoveTo self "0, 0, 0" Pawn 5.0 false))
    (:then_1
      (Utilities|FlowControl|RetriggerableDelay (Variables|Default|GetTriggerDelay))
      (AI|AIMoveTo self (Variables|Default|GetStarting%20Location) 0 5.0 false))))

(event Custom|OnEndBattle_Event
  (EventDispatchers|UnbindEventfromOnEndBattle (Variables|Default|GetBattle%20Scene) (delegate Custom|OnEndBattle_Event))
  (Actor|DestroyActor))

(event EventBeginPlay
  (Variables|Default|SetStarting%20Location (Transformation|GetActorLocation)))

(event Collision|EventActorBeginOverlap
  (params (OtherActor :type Actor%20Object%20Reference))
  (bind _battle_scene (Variables|Default|GetBattle%20Scene))
  (Class|KismetSystemLibrary|IsObjectOfSoftClass OtherActor "/Game/ThirdPerson/Blueprints/BP_ThirdPersonCharacter.BP_ThirdPersonCharacter_C"
    (:True
      (bind _aspawn (Utilities|Casting|CastToPawn OtherActor))
      (EventDispatchers|BindEventtoOnEndBattle _battle_scene (delegate Custom|OnEndBattle_Event))
      (Default|StartBattle _battle_scene _aspawn))))

(event EventTick
  (params (DeltaSeconds :type Float%20%28single-precision%29)))

(fn ConstructionScript)