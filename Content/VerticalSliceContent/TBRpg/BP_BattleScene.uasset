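; Possessable battle scene pawn that runs a turn-based RPG encounter from start to XP award or game quit on party defeat.
; Teleports the party into slots and async-spawns three enemies from a weighted-random encounter table row.
; Speed-sorted turns run through each actor's turn-based component, advancing on TurnEnded and skipping the dead.
; Player turns take an ability from the battle HUD, with debug keys for targeting, confirm and cancel.
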(event Custom|StartBattle
  (params (ReturnCharacter :type Pawn%20Object%20Reference))
  (Variables|Default|SetStopBattle false)
  (Initializers|InitializeStartBattle ReturnCharacter)
  (Variables|/Script/Engine.PlayerController|SetbShowMouseCursor (Variables|Default|GetPlayer%20Controller) true))

(event Custom|MovePartyToBattle
  (Initializers|InitializeMovePartytoBattleScene))

(event Custom|PlayerActorKilled_Event
  (params (ActorKilled :type Actor%20Object%20Reference))
  (CombatState|LoseBattle))

(event Custom|SpawnEnemies
  (bind _out_row (Initializers|PickEnemyLayout))
  (bind _class (Utilities|AsyncLoadClassAsset (.enemyclass1 _out_row))
    (:Completed
      (Initializers|InitializeEnemyParty _class (Variables|Default|GetEnemy1))
      (bind _class_2 (Utilities|AsyncLoadClassAsset (.enemyclass2 _out_row))
        (:Completed
          (Initializers|InitializeEnemyParty _class_2 (Variables|Default|GetEnemy2))
          (bind _class_3 (Utilities|AsyncLoadClassAsset (.enemyclass3 _out_row))
            (:Completed
              (Initializers|InitializeEnemyParty _class_3 (Variables|Default|GetEnemy3))
              (Setters|SetTurnOrder)
              (CallFunction|NextCharacter))))))))

(event Custom|NextCharacter
  (if (not (Variables|Default|GetStopBattle))
    (bind _targetedactor (Variables|Default|GetTargetedActor)
      (:then
        (Class|BPITurnBasedCombat|SetTargeted(Message) _targetedactor true))
      (:else
        _))
    (if (PureFunctions|IsTurnOrderComplete)
      (Variables|Default|SetTurnOrderIndex 0)
      (Setters|SetTurnOrder)
      (CallFunction|NextCharacter)
      (else
        (bind _component (Class|BPITurnBasedCombat|GetTurnBasedComponent(Message) (Utilities|Array|Get(acopy) (Variables|Default|GetTurnOrderActors) (Variables|Default|GetTurnOrderIndex))))
        (bind _currentvaluewithmod (Default|GetAttributeCurrent _component "HP"))
        (if (> _currentvaluewithmod 0.0)
          (Class|BPITurnBasedCombat|SetTurnActive(Message) (Variables|Default|GetActiveActor) false)
          (bind _output_get (Variables|Default|SetActiveActor (Utilities|Array|Get(acopy) (Variables|Default|GetTurnOrderActors) (Variables|Default|GetTurnOrderIndex))))
          (Class|BPITurnBasedCombat|SetTurnActive(Message) _output_get true)
          (Math|Integer|IncrementInt (Variables|Default|GetTurnOrderIndex)
            (:%20%20
              (bind _component_2 (Class|BPITurnBasedCombat|GetTurnBasedComponent(Message) (Variables|Default|GetActiveActor)))
              (EventDispatchers|BindEventtoTurnEnded _component_2 (delegate Custom|TurnEnded))
              (Default|StartTurn _component_2)
              (bind _output_get_2 (Variables|Default|SetbIsPlayerTurn (PureFunctions|IsAPlayerTurn)))
              (if _output_get_2
                (Default|SetPlayerInfo (Variables|Default|GetHUD) (Variables|Default|GetActiveActor))
                (EventDispatchers|BindEventtoOnAbilityChosen (Variables|Default|GetHUD) (delegate Custom|AbilityChosen_Event)))))
          (else
            (Math|Integer|IncrementInt (Variables|Default|GetTurnOrderIndex)
              (:%20%20
                (CallFunction|NextCharacter)))))))))

(event Custom|SetPlayerMenu
  (Default|SetPlayerInfo (Variables|Default|GetHUD) (Variables|Default|GetActiveActor))
  (EventDispatchers|BindEventtoOnAbilityChosen (Variables|Default|GetHUD) (delegate Custom|AbilityChosen_Event)))

(event Custom|AbilityChosen_Event
  (params (Ability :type BP%20Turn%20Based%20Ability%20Object%20Reference))
  (EventDispatchers|UnbindEventfromOnAbilityChosen (Variables|Default|GetHUD) (delegate Custom|AbilityChosen_Event))
  (bind _component (Class|BPITurnBasedCombat|GetTurnBasedComponent(Message) (Variables|Default|GetActiveActor)))
  (Variables|Default|SetOwnPartySelected (PureFunctions|IsPartyMemberSelected _component))
  (Setters|SetSelectionbyIndex (PureFunctions|GetArrayIndexinBattleScene _component))
  (bind _output_get (Variables|Default|SetCurrentAbility Ability))
  (bind _output (Default|UpdateSelectedTarget _output_get (Variables|/Game/VerticalSliceContent/TBRpg/TBRPG_PlayerController.TBRPG_PlayerController_C|GetActiveParty (Variables|Default|GetPlayer%20Controller)) (Variables|Default|GetEnemyParty) (Variables|Default|GetTargetedActor)))
  (Utilities|IsValid _output
    (:Is%20Valid
      (Setters|SetNewSelectedTarget _output)
      (Default|ClearUI (Variables|Default|GetHUD)))
    (:Is%20Not%20Valid
      (CallFunction|SetPlayerMenu))))

(event Custom|TurnEnded
  (Utilities|FlowControl|DelayUntilNextTick)
  (CallFunction|NextCharacter))

(event Custom|ActorKilled_Event
  (params (Actor :type Actor%20Object%20Reference))
  (Class|BPITurnBasedCombat|SetTargeted(Message) Actor false)
  (Utilities|Array|RemoveItem (Variables|Default|GetEnemyParty) Actor)
  (bind _asbp_tbenemy (Utilities|Casting|CastToBP_TBEnemy Actor))
  (CombatState|AddXptoAward (Variables|/Game/VerticalSliceContent/TBRpg/Characters/Enemies/BP_TBEnemy.BP_TBEnemy_C|GetXpOnDeath _asbp_tbenemy))
  (Actor|DestroyActor Actor)
  (if (not (> (Utilities|Array|Length (Variables|Default|GetEnemyParty)) 0))
    (CallFunction|EndBattle)))

(event Custom|EndBattle
  (Variables|Default|SetStopBattle true)
  (Variables|/Script/Engine.PlayerController|SetbShowMouseCursor (Game|GetPlayerController 0) false)
  (CallFunction|AwardPostCombatXP)
  (Default|CallOnEndBattle))

(event Custom|CancelAbility
  (Actor|DestroyActor (Variables|Default|GetCurrentAbility))
  (CallFunction|SetPlayerMenu)
  (Class|BPITurnBasedCombat|SetTargeted(Message) (Variables|Default|GetTargetedActor) false))

(event Input|KeyboardEvents|DebugKeyW
  (params (Key :type Key%20Structure) (ActionValue :type Input%20Action%20Value%20Structure))
  (:Pressed
    (if (Variables|Default|GetbIsPlayerTurn)
      (bind _currentability (Variables|Default|GetCurrentAbility)
        (:then
          (bind _output (Default|SelectUp _currentability (Variables|/Game/VerticalSliceContent/TBRpg/TBRPG_PlayerController.TBRPG_PlayerController_C|GetActiveParty (Variables|Default|GetPlayer%20Controller)) (Variables|Default|GetEnemyParty) (Variables|Default|GetTargetedActor)))
          (Setters|SetNewSelectedTarget _output))
        (:else)))))

(event Input|KeyboardEvents|DebugKeyA
  (params (Key :type Key%20Structure) (ActionValue :type Input%20Action%20Value%20Structure))
  (:Pressed
    (if (Variables|Default|GetbIsPlayerTurn)
      (bind _currentability (Variables|Default|GetCurrentAbility)
        (:then
          (bind _output (Default|SelectOtherParty _currentability (Variables|/Game/VerticalSliceContent/TBRpg/TBRPG_PlayerController.TBRPG_PlayerController_C|GetActiveParty (Variables|Default|GetPlayer%20Controller)) (Variables|Default|GetEnemyParty) (Variables|Default|GetTargetedActor)))
          (Setters|SetNewSelectedTarget _output))
        (:else)))))

(event Input|KeyboardEvents|DebugKeyS
  (params (Key :type Key%20Structure) (ActionValue :type Input%20Action%20Value%20Structure))
  (:Pressed
    (if (Variables|Default|GetbIsPlayerTurn)
      (bind _currentability (Variables|Default|GetCurrentAbility)
        (:then
          (bind _output (Default|SelectDown _currentability (Variables|/Game/VerticalSliceContent/TBRpg/TBRPG_PlayerController.TBRPG_PlayerController_C|GetActiveParty (Variables|Default|GetPlayer%20Controller)) (Variables|Default|GetEnemyParty) (Variables|Default|GetTargetedActor)))
          (Setters|SetNewSelectedTarget _output))
        (:else)))))

(event Input|KeyboardEvents|DebugKeyD
  (params (Key :type Key%20Structure) (ActionValue :type Input%20Action%20Value%20Structure))
  (:Pressed
    (if (Variables|Default|GetbIsPlayerTurn)
      (bind _currentability (Variables|Default|GetCurrentAbility)
        (:then
          (bind _output (Default|SelectOtherParty (stale Input|KeyboardEvents|DebugKeyA _currentability) (Variables|/Game/VerticalSliceContent/TBRpg/TBRPG_PlayerController.TBRPG_PlayerController_C|GetActiveParty (Variables|Default|GetPlayer%20Controller)) (Variables|Default|GetEnemyParty) (Variables|Default|GetTargetedActor)))
          (Setters|SetNewSelectedTarget _output))
        (:else)))))

(event Input|KeyboardEvents|DebugKeyEnter
  (params (Key :type Key%20Structure) (ActionValue :type Input%20Action%20Value%20Structure))
  (:Pressed
    (if (Variables|Default|GetbIsPlayerTurn)
      (bind _component (Class|BPITurnBasedCombat|GetTurnBasedComponent(Message) (Variables|Default|GetActiveActor)))
      (Default|ActivateQueuedAbilities _component))))

(event Input|KeyboardEvents|DebugKeyBackspace
  (params (Key :type Key%20Structure) (ActionValue :type Input%20Action%20Value%20Structure))
  (:Pressed
    (Actor|DestroyActor (Variables|Default|GetCurrentAbility))
    (CallFunction|SetPlayerMenu)
    (Class|BPITurnBasedCombat|SetTargeted(Message) (Variables|Default|GetTargetedActor) false)))

(event Input|KeyboardEvents|DebugKeyUp
  (params (Key :type Key%20Structure) (ActionValue :type Input%20Action%20Value%20Structure)))

(event Input|KeyboardEvents|DebugKeyDown
  (params (Key :type Key%20Structure) (ActionValue :type Input%20Action%20Value%20Structure)))

(event Input|KeyboardEvents|DebugKeyLeft
  (params (Key :type Key%20Structure) (ActionValue :type Input%20Action%20Value%20Structure)))

(event Input|KeyboardEvents|DebugKeyRight
  (params (Key :type Key%20Structure) (ActionValue :type Input%20Action%20Value%20Structure)))

(fn ConstructionScript)

(fn GetBattleCharacters
  (LocalVariables|SetOutputArray (Variables|/Game/VerticalSliceContent/TBRpg/TBRPG_PlayerController.TBRPG_PlayerController_C|GetActiveParty (Variables|Default|GetPlayer%20Controller)))
  (for _array_element (Variables|Default|GetEnemyParty)
    (Utilities|Array|AddUnique (LocalVariables|GetOutputArray) _array_element))
  (return (LocalVariables|GetOutputArray)))

(fn PickEnemyLayout
  (if (Utilities|IsValid (Variables|Default|GetEncounterRate))
    (if (== (Class|DataTableFunctionLibrary|GetDataTableRowStruct (Variables|Default|GetEncounterRate)) "/Game/VerticalSliceContent/TBRpg/Structs/EnemyEncounter.EnemyEncounter")
      (bind _outrownames (DataTable|GetDataTableRowNames (Variables|Default|GetEncounterRate)))
      (for _array_element _outrownames
        (bind _returnvalue (Utilities|GetDataTableRow (Variables|Default|GetEncounterRate) _array_element)
          (:then
            (LocalVariables|SetTotalWeight (+ (LocalVariables|GetTotalWeight) (.Weight (Utilities|Struct|BreakEnemyEncounter _returnvalue)))))))
      (LocalVariables|SetTargetWeight (Math|Random|RandomFloatinRange 0.0 (LocalVariables|GetTotalWeight)))
      (bind _outrownames_2 (DataTable|GetDataTableRowNames "/Game/VerticalSliceContent/TBRpg/DataAssets/BasicEncounter.BasicEncounter"))
      (for _array_element_2 _outrownames_2
        (bind _returnvalue_2 (Utilities|GetDataTableRow (Variables|Default|GetEncounterRate) _array_element_2)
          (:then
            (bind _output_get (LocalVariables|SetCOuntUpWeight (+ (LocalVariables|GetCOuntUpWeight) (.Weight (Utilities|Struct|BreakEnemyEncounter _returnvalue_2)))))
            (if (<= (LocalVariables|GetTargetWeight) _output_get)
              (return _returnvalue_2)))))
      (else
        (Development|PrintString "No valid Encounter Table")
        (return "")))
    (else
      (Development|PrintString "Missing Encounter Table")
      (return ""))))

(fn SetTurnOrder
  (for _array_element (Getters|GetBattleCharacters)
    (bind _component (Class|BPITurnBasedCombat|GetTurnBasedComponent(Message) _array_element))
    (bind _currentvaluewithmod (Default|GetAttributeCurrent _component "Speed"))
    (Utilities|Array|Add (LocalVariables|GetSpeeds) _currentvaluewithmod))
  (Class|KismetArrayLibrary|SortFloatArray (LocalVariables|GetSpeeds) false "Descending")
  (for _array_element_2 (LocalVariables|GetSpeeds)
    (for _array_element_3 (Getters|GetBattleCharacters)
      (bind _component_2 (Class|BPITurnBasedCombat|GetTurnBasedComponent(Message) _array_element_3))
      (bind _currentvaluewithmod_2 (Default|GetAttributeCurrent _component_2 "Speed"))
      (if (== _array_element_2 _currentvaluewithmod_2)
        (Utilities|Array|AddUnique (LocalVariables|GetTurnOrder) _array_element_3))))
  (Variables|Default|SetTurnOrderActors (LocalVariables|GetTurnOrder)))

(fn SetSelectionbyIndex
  (params (Index :type Integer))
  (if (Variables|Default|GetOwnPartySelected)
    (Setters|SetSelectioninArray Index (Variables|/Game/VerticalSliceContent/TBRpg/TBRPG_PlayerController.TBRPG_PlayerController_C|GetActiveParty (Variables|Default|GetPlayer%20Controller)))
    (else
      (Setters|SetSelectioninArray Index (Variables|Default|GetEnemyParty)))))

(fn SetSelectioninArray
  (params (Index :type Integer) (Array :type Array%20of%20Actor%20Object%20References))
  (bind _returnvalue (Utilities|Array|LastIndex Array))
  (if (> Index _returnvalue)
    (Variables|Default|SetSelectionIndex 0)
    (elif (< Index 0)
      (Variables|Default|SetSelectionIndex _returnvalue)
      (else
        (Variables|Default|SetSelectionIndex Index))))
  (Variables|Default|SetTargetedActor (Utilities|Array|Get(acopy) Array (Variables|Default|GetSelectionIndex))))

(fn SetNewSelectedTarget
  (params (Actor :type Actor%20Object%20Reference))
  (Utilities|IsValid Actor
    (:Is%20Valid
      (Class|BPITurnBasedCombat|SetTargeted(Message) Actor true)
      (Class|BPITurnBasedCombat|SetTargeted(Message) (Variables|Default|GetTargetedActor) false)
      (Variables|Default|SetTargetedActor Actor)
      (Setters|SetNewPartyMemberTarget (Utilities|Array|FindItem (Variables|/Game/VerticalSliceContent/TBRpg/TBRPG_PlayerController.TBRPG_PlayerController_C|GetActiveParty (Variables|Default|GetPlayer%20Controller)) (Variables|Default|GetActiveActor)) Actor)
      (Default|SetTargetInfo (Variables|Default|GetHUD) (Variables|Default|GetTargetedActor)))))

(fn SetNewPartyMemberTarget
  (params (PartyMemberIndex :type Integer) (NewTarget :type Actor%20Object%20Reference))
  (bind _component (Class|BPITurnBasedCombat|GetTurnBasedComponent(Message) (Utilities|Array|Get(acopy) (Variables|/Game/VerticalSliceContent/TBRpg/TBRPG_PlayerController.TBRPG_PlayerController_C|GetActiveParty (Variables|Default|GetPlayer%20Controller)) PartyMemberIndex)))
  (Variables|/Game/VerticalSliceContent/TBRpg/Components/AbilitySystemComponent.AbilitySystemComponent_C|SetTarget _component NewTarget))

(fn InitializeEnemyParty
  (params (Class :type Object%20Class%20Reference) (Location :type Billboard%20Component%20Object%20Reference))
  (bind _asactor (Utilities|Casting|CastToActorClass Class)
    (:then
      (bind _returnvalue (Game|SpawnActorfromClass _asactor (Transformation|GetWorldTransform Location) "Undefined" "MultiplyWithRoot" 0 0))
      (bind _output_get (LocalVariables|SetSpawnedActor _returnvalue))
      (Utilities|Array|AddUnique (Variables|Default|GetEnemyParty) _output_get)
      (Setters|SetNewPartyMemberTarget 0 (LocalVariables|GetSpawnedActor))
      (bind _component (Class|BPITurnBasedCombat|GetTurnBasedComponent(Message) (LocalVariables|GetSpawnedActor)))
      (EventDispatchers|BindEventtoActorKilled _component (EventDispatchers|CreateEvent :!event Custom|ActorKilled_Event)))
    (:CastFailed
      (Development|PrintString (Utilities|String|Append "Failed to Cast Actor: \"" (Utilities|GetClassDisplayName Class) "\" to class") true true "(R=0.234375,G=0.000000,B=0.061145,A=1.000000)"))))

(fn InitializeMovePartytoBattleScene
  (bind _astbrpg_player_controller (Utilities|Casting|CastToTBRPG_PlayerController (Game|GetPlayerController 0)))
  (bind _output_get (Variables|Default|SetPlayer%20Controller _astbrpg_player_controller))
  (for (_array_element _array_index) (Variables|/Game/VerticalSliceContent/TBRpg/TBRPG_PlayerController.TBRPG_PlayerController_C|GetActiveParty _output_get)
    (Transformation|SetActorTransform _array_element (Transformation|GetWorldTransform (Utilities|Array|Get(acopy) (Utilities|Array|MakeArray (Variables|Default|GetPlayer1) (Variables|Default|GetPlayer2) (Variables|Default|GetPlayer3)) _array_index)))
    (Rendering|SetActorHiddenInGame _array_element false)
    (bind _component (Class|BPITurnBasedCombat|GetTurnBasedComponent(Message) _array_element))
    (EventDispatchers|BindEventtoActorKilled _component (EventDispatchers|CreateEvent :!event Custom|PlayerActorKilled_Event))))

(fn InitializeStartBattle
  (params (ReturnCharacter :type Pawn%20Object%20Reference))
  (Variables|Default|SetReturnCharacter ReturnCharacter)
  (Rendering|SetActorHiddenInGame false)
  (CallFunction|MovePartytoBattle)
  (CallFunction|SpawnEnemies)
  (Pawn|Possess (Game|GetPlayerController 0) self)
  (bind _returnvalue (UserInterface|CreateWidget "/Game/VerticalSliceContent/TBRpg/UI/BattleHUD.BattleHUD_C"))
  (bind _output_get (Variables|Default|SetHUD _returnvalue))
  (UserInterface|Viewport|AddtoViewport _output_get 0))

(fn LoseBattle
  (for _array_element (Variables|/Game/VerticalSliceContent/TBRpg/TBRPG_PlayerController.TBRPG_PlayerController_C|GetActiveParty (Variables|Default|GetPlayer%20Controller))
    (bind _component (Class|BPITurnBasedCombat|GetTurnBasedComponent(Message) _array_element))
    (bind _currentvaluewithmod (Default|GetAttributeCurrent _component "HP"))
    (if (> _currentvaluewithmod 0.0)
      (return)))
  (Variables|Default|SetStopBattle true)
  (Game|QuitGame 0 "Quit" false))

(fn AddXptoAward
  (params (XP :type Integer))
  (bind _xpreward (Variables|Default|GetXpReward))
  (for _array_element (Variables|/Game/VerticalSliceContent/TBRpg/TBRPG_PlayerController.TBRPG_PlayerController_C|GetActiveParty (Variables|Default|GetPlayer%20Controller))
    (bind _component (Class|BPITurnBasedCombat|GetTurnBasedComponent(Message) _array_element))
    (bind _currentvaluewithmod (Default|GetAttributeCurrent _component "HP"))
    (if (> _currentvaluewithmod 0.0)
      (if (.ReturnValue (Utilities|Map|Find _xpreward _array_element))
        (Variables|Default|SetPreviousValue (.Value (Utilities|Map|Find _xpreward _array_element)))
        (else
          (Variables|Default|SetPreviousValue 0)))
      (Utilities|Map|Add _xpreward _array_element (+ XP (Variables|Default|GetPreviousValue))))))

(fn AwardXp
  (bind _xpreward (Variables|Default|GetXpReward))
  (bind _keys (Utilities|Map|Keys _xpreward))
  (for _array_element _keys
    (bind _asbp_tbplayer (Utilities|Casting|CastToBP_TBPlayer _array_element))
    (if (.ReturnValue (Utilities|Map|Find _xpreward _array_element))
      (bind _component (Class|BPITurnBasedCombat|GetTurnBasedComponent(Message) _asbp_tbplayer))
      (bind _currentvaluewithmod (Default|GetAttributeCurrent _component "HP"))
      (if (> _currentvaluewithmod 0.0)
        (Default|GiveXp _asbp_tbplayer (.Value (Utilities|Map|Find _xpreward _array_element)))))))

(fn IsTurnOrderComplete
  (if (>= (Variables|Default|GetTurnOrderIndex) (Utilities|Array|Length (Variables|Default|GetTurnOrderActors)))
    (return true)
    (else
      (return false))))

(fn IsAPlayerTurn
  (return (Utilities|Array|ContainsItem (Variables|/Game/VerticalSliceContent/TBRpg/TBRPG_PlayerController.TBRPG_PlayerController_C|GetActiveParty (Variables|Default|GetPlayer%20Controller)) (Variables|Default|GetActiveActor))))

(fn IsPartyMemberSelected
  (params (OwningAbilitySystemComponent :type Ability%20System%20Component%20Object%20Reference))
  (return (Utilities|Array|ContainsItem (Variables|/Game/VerticalSliceContent/TBRpg/TBRPG_PlayerController.TBRPG_PlayerController_C|GetActiveParty (Variables|Default|GetPlayer%20Controller)) (Variables|/Game/VerticalSliceContent/TBRpg/Components/AbilitySystemComponent.AbilitySystemComponent_C|GetTarget OwningAbilitySystemComponent))))

(fn GetArrayIndexinBattleScene
  (params (AbilitySystemComponent :type Ability%20System%20Component%20Object%20Reference))
  (return (Math|Integer|SelectInt (Utilities|Array|FindItem (Variables|/Game/VerticalSliceContent/TBRpg/TBRPG_PlayerController.TBRPG_PlayerController_C|GetActiveParty (Variables|Default|GetPlayer%20Controller)) (Variables|/Game/VerticalSliceContent/TBRpg/Components/AbilitySystemComponent.AbilitySystemComponent_C|GetTarget AbilitySystemComponent)) (Utilities|Array|FindItem (Variables|Default|GetEnemyParty) (Variables|/Game/VerticalSliceContent/TBRpg/Components/AbilitySystemComponent.AbilitySystemComponent_C|GetTarget AbilitySystemComponent)) (PureFunctions|IsPartyMemberSelected AbilitySystemComponent))))

(fn AwardPostCombatXP
  (CombatState|AwardXp)
  (Rendering|SetActorHiddenInGame true)
  (for _array_element (Getters|GetBattleCharacters)
    (Rendering|SetActorHiddenInGame _array_element true)
    (bind _component (Class|BPITurnBasedCombat|GetTurnBasedComponent(Message) _array_element))
    (EventDispatchers|UnbindallEventsfromTurnEnded _component)
    (Class|BPITurnBasedCombat|SetTurnActive(Message) _array_element false)
    (Class|BPITurnBasedCombat|SetTargeted(Message) _array_element false))
  (Pawn|Possess (Game|GetPlayerController 0) (Variables|Default|GetReturnCharacter))
  (Widget|RemovefromParent (Variables|Default|GetHUD)))