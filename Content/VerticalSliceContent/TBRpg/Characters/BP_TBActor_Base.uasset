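; Base character actor for a turn-based RPG, exposing its AbilitySystemComponent through GetTurnBasedComponent.
; On BeginPlay it applies a small random Speed effect to itself through that component, so each instance's stat varies.
; SetTurnActive and SetTargeted show state by swapping skeletal mesh overlay materials for turn and selection outlines.
; Untargeting restores the turn outline if the component reports it is still this actor's turn, otherwise it clears the overlay.
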(event EventBeginPlay
  (Default|ApplyEffecttoSelf (Variables|Default|GetAbilitySystemComponent) "Speed" (Math|Random|RandomFloatinRange -2.0 2.0) "NewEnumerator0" "NewEnumerator4" "NewEnumerator0"))

(event Collision|EventActorBeginOverlap
  (params (OtherActor :type Actor%20Object%20Reference)))

(event EventTick
  (params (DeltaSeconds :type Float%20%28single-precision%29)))

(event EventSetTargeted
  (params (IsTargeted :type Boolean))
  (if IsTargeted
    (Rendering|Material|SetOverlayMaterial (Variables|Default|GetSkeletalMesh) "/Game/VerticalSliceContent/TBRpg/Characters/SelectionOutline.SelectionOutline" :!class /Script/Engine.MeshComponent)
    (elif (Variables|/Game/VerticalSliceContent/TBRpg/Components/AbilitySystemComponent.AbilitySystemComponent_C|GetIsTurn (Variables|Default|GetAbilitySystemComponent))
      (Rendering|Material|SetOverlayMaterial (Variables|Default|GetSkeletalMesh) "/Game/VerticalSliceContent/TBRpg/Characters/TurnOutline.TurnOutline" :!class /Script/Engine.MeshComponent)
      (else
        (Rendering|Material|SetOverlayMaterial (Variables|Default|GetSkeletalMesh) 0 :!class /Script/Engine.MeshComponent)))))

(event EventSetTurnActive
  (params (IsActive :type Boolean))
  (if IsActive
    (Rendering|Material|SetOverlayMaterial (Variables|Default|GetSkeletalMesh) "/Game/VerticalSliceContent/TBRpg/Characters/TurnOutline.TurnOutline" :!class /Script/Engine.MeshComponent)
    (else
      (Rendering|Material|SetOverlayMaterial (Variables|Default|GetSkeletalMesh) 0 :!class /Script/Engine.MeshComponent))))

(fn ConstructionScript)

(fn GetTurnBasedComponent
  (return (Variables|Default|GetAbilitySystemComponent)))