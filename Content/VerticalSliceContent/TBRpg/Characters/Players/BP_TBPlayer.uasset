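; BP_TBPlayer is a player character for the turn-based RPG, granted Attack and Wait abilities and set to level 1 on BeginPlay.
; GiveXp accumulates experience and uses an XP curve to decide when to call LevelUp.
; LevelUp reads HP for the new level from a curve and applies it as two effects on different HP stats through its ability system component.
; GetTurnBasedComponent exposes that same component.
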(event EventBeginPlay
  (bind _abilitysystemcomponent (Variables|Default|GetAbilitySystemComponent))
  (|CallParentFunction)
  (Default|GiveAbility _abilitysystemcomponent "/Game/VerticalSliceContent/TBRpg/GameplayAbilities/GA_Attack.GA_Attack_C")
  (Default|GiveAbility _abilitysystemcomponent "/Game/VerticalSliceContent/TBRpg/GameplayAbilities/GA_Wait.GA_Wait_C")
  (CallFunction|LevelUp 1))

(event Collision|EventActorBeginOverlap
  (params (OtherActor :type Actor%20Object%20Reference))
  (|CallParentFunction OtherActor) ; This node is disabled and will not be called.\nDrag off pins to build functionality.
)

(event EventTick
  (params (DeltaSeconds :type Float%20%28single-precision%29))
  (|CallParentFunction DeltaSeconds))

(fn ConstructionScript
  (|CallParentFunction))

(fn GiveXp
  (params (XP :type Integer))
  (bind _output_get (Variables|Default|SetTotalExperience (+ XP (Variables|Default|GetTotalExperience))))
  (if (> (Math|Float|Floor (Math|Curves|GetFloatValue (Variables|Default|GetXpCurve) (Math|Conversions|ToFloat(Integer) _output_get))) (Variables|Default|GetCurrentLevel))
    (CallFunction|LevelUp (Math|Float|Floor (Math|Curves|GetFloatValue (Variables|Default|GetXpCurve) (Math|Conversions|ToFloat(Integer) _output_get))))))

(fn LevelUp
  (params (NewLevel :type Integer))
  (bind _abilitysystemcomponent (Variables|Default|GetAbilitySystemComponent))
  (bind _output_get (Variables|Default|SetCurrentLevel NewLevel))
  (Default|ApplyEffecttoSelf _abilitysystemcomponent "HP" (Math|Curves|GetFloatValue (Variables|Default|GetHpCurve) (Math|Conversions|ToFloat(Integer) _output_get)) "NewEnumerator0" "NewEnumerator2" "NewEnumerator3")
  (Default|ApplyEffecttoSelf _abilitysystemcomponent "HP" (Math|Curves|GetFloatValue (Variables|Default|GetHpCurve) (Math|Conversions|ToFloat(Integer) _output_get)) "NewEnumerator0" "NewEnumerator4" "NewEnumerator3"))

(fn GetTurnBasedComponent
  (return (Variables|Default|GetAbilitySystemComponent)))