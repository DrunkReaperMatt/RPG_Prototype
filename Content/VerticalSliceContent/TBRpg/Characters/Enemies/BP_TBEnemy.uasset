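; Enemy character Blueprint for the turn-based RPG, with turn behavior driven by a StateTree.
; On BeginPlay it grants GA_Wait to its ability system component, which also serves as its turn-based component.
; That component's TurnStarted event starts the StateTree logic.
; SetTurnActive is empty, and a disconnected branch that activates Wait and prints a debug message never runs.
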(event TurnStarted(AbilitySystemComponent)
  (AI|Logic|StartLogic (Variables|Default|GetStateTree)))

(event EventSetTurnActive
  (params (IsActive :type Boolean)))

(event Collision|EventActorBeginOverlap
  (params (OtherActor :type Actor%20Object%20Reference))
  (|CallParentFunction OtherActor))

(event EventTick
  (params (DeltaSeconds :type Float%20%28single-precision%29))
  (|CallParentFunction DeltaSeconds))

(event EventBeginPlay
  (|CallParentFunction)
  (Default|GiveAbility (Variables|Default|GetAbilitySystemComponent) "/Game/VerticalSliceContent/TBRpg/GameplayAbilities/GA_Wait.GA_Wait_C"))

(fn ConstructionScript)

(fn GetTurnBasedComponent
  (return (Variables|Default|GetAbilitySystemComponent)))