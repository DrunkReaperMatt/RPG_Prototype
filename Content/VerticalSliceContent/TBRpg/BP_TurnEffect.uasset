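; Turn-based RPG effect that changes one named attribute on a target component by a chosen stat field and math operation.
; ApplyEffect handles instant, turn-counted, infinite and temporary types, and EndEffect removes it from the target's active effects.
; DoEffect writes the result and calls an attribute update, recording AbsoluteChange so temporary effects can undo it.
; Multiply squares the current value, ignoring Magnitude, and Override records its change with reversed sign.
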(event Custom|ApplyEffect
  (switch Utilities|FlowControl|Switch|SwitchonEffectType (Variables|Default|GetEffectType)
    (:NewEnumerator0
      (CallFunction|DoEffect)
      (CallFunction|EndEffect))
    (:NewEnumerator1
      (CallFunction|DoEffect)
      (bind _result (Math|Integer|DecrementInt (Variables|Default|GetEffectTurnCounter))
        (:%20%20
          (if (<= _result 0)
            (CallFunction|EndEffect)))))
    (:NewEnumerator2
      (CallFunction|DoEffect))
    (:NewEnumerator3
      (CallFunction|DoEffect))))

(event Custom|EndEffect
  (switch Utilities|FlowControl|Switch|SwitchonEffectType (Variables|Default|GetEffectType)
    (:NewEnumerator0
      _)
    (:NewEnumerator1
      _)
    (:NewEnumerator2
      _)
    (:NewEnumerator3
      (Variables|Default|SetEffectMath "NewEnumerator0")
      (Variables|Default|SetMagnitude (* (Variables|Default|GetAbsoluteChange) -1.0))
      (CallFunction|DoEffect)))
  (bind _targetcomponent (Variables|Default|GetTargetComponent)
    (:then
      (Utilities|Array|RemoveItem (Variables|/Game/VerticalSliceContent/TBRpg/Components/AbilitySystemComponent.AbilitySystemComponent_C|GetActiveEffects _targetcomponent) self))
    (:else)))

(fn DoEffect
  (bind _targetcomponent (Variables|Default|GetTargetComponent)
    (:then
      (for (_array_element _array_index) (Variables|/Game/VerticalSliceContent/TBRpg/Components/AbilitySystemComponent.AbilitySystemComponent_C|GetAttributes _targetcomponent)
        (if (== (.name _array_element) (Variables|Default|GetAttributeToEffect))
          (switch Utilities|FlowControl|Switch|SwitchonTargetStat (Variables|Default|GetTargetStat)
            (:NewEnumerator0
              (bind _newvalue (CallFunction|CalculateNewValue (.MinValue (Utilities|Struct|BreakStat (.stat (Utilities|Array|Get(acopy) (Variables|/Game/VerticalSliceContent/TBRpg/Components/AbilitySystemComponent.AbilitySystemComponent_C|GetAttributes _targetcomponent) _array_index))))))
              (Utilities|Struct|SetmembersinStat (.stat (Utilities|Array|Get(acopy) (Variables|/Game/VerticalSliceContent/TBRpg/Components/AbilitySystemComponent.AbilitySystemComponent_C|GetAttributes _targetcomponent) _array_index)) _newvalue))
            (:NewEnumerator1
              (bind _newvalue_2 (CallFunction|CalculateNewValue (.MinValueMod (Utilities|Struct|BreakStat (.stat (Utilities|Array|Get(acopy) (Variables|/Game/VerticalSliceContent/TBRpg/Components/AbilitySystemComponent.AbilitySystemComponent_C|GetAttributes _targetcomponent) _array_index))))))
              (Utilities|Struct|SetmembersinStat (.stat (Utilities|Array|Get(acopy) (Variables|/Game/VerticalSliceContent/TBRpg/Components/AbilitySystemComponent.AbilitySystemComponent_C|GetAttributes _targetcomponent) _array_index)) _newvalue_2))
            (:NewEnumerator2
              (bind _newvalue_3 (CallFunction|CalculateNewValue (.MaxValue (Utilities|Struct|BreakStat (.stat (Utilities|Array|Get(acopy) (Variables|/Game/VerticalSliceContent/TBRpg/Components/AbilitySystemComponent.AbilitySystemComponent_C|GetAttributes _targetcomponent) _array_index))))))
              (Utilities|Struct|SetmembersinStat (.stat (Utilities|Array|Get(acopy) (Variables|/Game/VerticalSliceContent/TBRpg/Components/AbilitySystemComponent.AbilitySystemComponent_C|GetAttributes _targetcomponent) _array_index)) _newvalue_3))
            (:NewEnumerator3
              (bind _newvalue_4 (CallFunction|CalculateNewValue (.MaxValueMod (Utilities|Struct|BreakStat (.stat (Utilities|Array|Get(acopy) (Variables|/Game/VerticalSliceContent/TBRpg/Components/AbilitySystemComponent.AbilitySystemComponent_C|GetAttributes _targetcomponent) _array_index))))))
              (Utilities|Struct|SetmembersinStat (.stat (Utilities|Array|Get(acopy) (Variables|/Game/VerticalSliceContent/TBRpg/Components/AbilitySystemComponent.AbilitySystemComponent_C|GetAttributes _targetcomponent) _array_index)) _newvalue_4))
            (:NewEnumerator4
              (bind _newvalue_5 (CallFunction|CalculateNewValue (.CurrentValue (Utilities|Struct|BreakStat (.stat (Utilities|Array|Get(acopy) (Variables|/Game/VerticalSliceContent/TBRpg/Components/AbilitySystemComponent.AbilitySystemComponent_C|GetAttributes _targetcomponent) _array_index))))))
              (Utilities|Struct|SetmembersinStat (.stat (Utilities|Array|Get(acopy) (Variables|/Game/VerticalSliceContent/TBRpg/Components/AbilitySystemComponent.AbilitySystemComponent_C|GetAttributes _targetcomponent) _array_index)) _newvalue_5))
            (:NewEnumerator5
              (bind _newvalue_6 (CallFunction|CalculateNewValue (.CurrentValueMod (Utilities|Struct|BreakStat (.stat (Utilities|Array|Get(acopy) (Variables|/Game/VerticalSliceContent/TBRpg/Components/AbilitySystemComponent.AbilitySystemComponent_C|GetAttributes _targetcomponent) _array_index))))))
              (Utilities|Struct|SetmembersinStat (.stat (Utilities|Array|Get(acopy) (Variables|/Game/VerticalSliceContent/TBRpg/Components/AbilitySystemComponent.AbilitySystemComponent_C|GetAttributes _targetcomponent) _array_index)) _newvalue_6)))
          (Default|CallUpdateAttribute (Utilities|Array|Get(acopy) (Variables|/Game/VerticalSliceContent/TBRpg/Components/AbilitySystemComponent.AbilitySystemComponent_C|GetAttributes _targetcomponent) _array_index))
          (return))))
    (:else)))

(fn CalculateNewValue
  (params (CurrentValue :type Float%20%28double-precision%29))
  (bind _magnitude (Variables|Default|GetMagnitude))
  (bind _returnvalue (+ _magnitude CurrentValue))
  (bind _returnvalue_2 (* CurrentValue CurrentValue))
  (bind _returnvalue_3 (/ CurrentValue _magnitude))
  (switch Utilities|FlowControl|Switch|SwitchonEffectMath (Variables|Default|GetEffectMath)
    (:NewEnumerator0
      (Variables|Default|SetAbsoluteChange (- _returnvalue CurrentValue))
      (return _returnvalue))
    (:NewEnumerator1
      (Variables|Default|SetAbsoluteChange (- _returnvalue_2 CurrentValue))
      (return _returnvalue_2))
    (:NewEnumerator2
      (Variables|Default|SetAbsoluteChange (- _returnvalue_3 CurrentValue))
      (return _returnvalue_3))
    (:NewEnumerator3
      (Variables|Default|SetAbsoluteChange (- CurrentValue (Variables|Default|GetMagnitude)))
      (return _magnitude))))