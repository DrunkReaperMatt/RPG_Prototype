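; GA_Attack is a basic attack ability for a turn-based RPG that damages the owning ability component's current target.
; On activation it commits, spawns a Niagara hit effect at the target and applies a fixed negative HP effect through the ability component.
; It prints the damage, then ends after a short delay; a failed commit only prints a missing-MP message without calling EndAbility.
; Target selection defers to the parent class.
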(event EventActivateAbility
  (bind _owningabilitycomponent (Variables|Default|GetOwningAbilityComponent))
  (bind _target (Variables|/Game/VerticalSliceContent/TBRpg/Components/AbilitySystemComponent.AbilitySystemComponent_C|GetTarget _owningabilitycomponent))
  (bind _commited (CallFunction|CommitAbility))
  (if _commited
    (bind _component (Class|BPITurnBasedCombat|GetTurnBasedComponent(Message) _target))
    (Niagara|SpawnSystematLocation "/Game/VerticalSliceContent/TBRpg/NS_AttackHit.NS_AttackHit" (Transformation|GetActorLocation _target))
    (bind _effectref (Default|ApplyEffecttoTarget (Variables|Default|GetOwningAbilityComponent) _component "HP" -3.0 "NewEnumerator0" "NewEnumerator4" "NewEnumerator0"))
    (Development|PrintString (Utilities|String|Append "Dealt " (Utilities|String|ToString(Float) (Math|Float|Absolute(Float) (Variables|/Game/VerticalSliceContent/TBRpg/BP_TurnEffect.BP_TurnEffect_C|GetMagnitude _effectref))) " to target :" (Utilities|GetDisplayName (Variables|/Game/VerticalSliceContent/TBRpg/BP_TurnEffect.BP_TurnEffect_C|GetTargetComponent _effectref))))
    (Utilities|FlowControl|Delay 3.0)
    (Development|PrintString "End attack")
    (CallFunction|EndAbility)
    (else
      (Development|PrintString "Missing MP"))))

(fn ConstructionScript
  (|CallParentFunction))

(fn CanSelect
  (params (Actor :type Actor%20Object%20Reference))
  (bind _canselect (|CallParentFunction Actor))
  (return _canselect))