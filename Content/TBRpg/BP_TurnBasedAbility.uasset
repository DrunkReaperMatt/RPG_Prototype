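; Base actor for turn-based RPG abilities, with empty activate and select hooks and an end event that notifies, then destroys it.
; CommitAbility checks affordability and applies the cost through the owning ability component, or destroys the actor.
; Targeting helpers step within or swap between player and enemy parties via a modulo-wrapped search filtered by CanSelect, which defaults to true.
; The countdown search's exit test stops it after one rejected candidate.
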(event Custom|ActivateAbility)

(event Custom|EndAbility
  (Default|CallAbilityEnd self)
  (Actor|DestroyActor))

(event Custom|SelectAbility)

(fn ConstructionScript)

(fn CommitAbility
  (bind _cost (Variables|Default|GetCost))
  (bind _cando (CallFunction|CanDoAbility (Variables|Default|GetOwningAbilityComponent) (Utilities|GetClass self)))
  (if _cando
    (Default|ApplyEffecttoSelf (Variables|Default|GetOwningAbilityComponent) (.name _cost) (* (.cost _cost) -1.0) "NewEnumerator0" "NewEnumerator4" "NewEnumerator0")
    (return true)
    (else
      (Actor|DestroyActor)
      (return false))))

(fn SelectUp
  (params (PlayerParty :type Array%20of%20Actor%20Object%20References) (EnemyParty :type Array%20of%20Actor%20Object%20References) (CurrentSelected :type Actor%20Object%20Reference))
  (if (Utilities|Array|ContainsItem PlayerParty CurrentSelected)
    (bind _output (CallFunction|LoopArraywithWrap PlayerParty true (- (Utilities|Array|FindItem PlayerParty CurrentSelected) 1)))
    (return _output)
    (else
      (bind _output_2 (CallFunction|LoopArraywithWrap EnemyParty true (- (Utilities|Array|FindItem EnemyParty CurrentSelected) 1)))
      (return _output_2))))

(fn SelectDown
  (params (PlayerParty :type Array%20of%20Actor%20Object%20References) (EnemyParty :type Array%20of%20Actor%20Object%20References) (CurrentSelected :type Actor%20Object%20Reference))
  (if (Utilities|Array|ContainsItem PlayerParty CurrentSelected)
    (bind _output (CallFunction|LoopArraywithWrap PlayerParty false (+ (Utilities|Array|FindItem PlayerParty CurrentSelected) 1)))
    (return _output)
    (else
      (bind _output_2 (CallFunction|LoopArraywithWrap EnemyParty false (+ (Utilities|Array|FindItem EnemyParty CurrentSelected) 1)))
      (return _output_2))))

(fn SelectOtherParty
  (params (PlayerParty :type Array%20of%20Actor%20Object%20References) (EnemyParty :type Array%20of%20Actor%20Object%20References) (CurrentSelected :type Actor%20Object%20Reference))
  (if (Utilities|Array|ContainsItem PlayerParty CurrentSelected)
    (bind _output (CallFunction|LoopArraywithWrap EnemyParty true (Utilities|Array|FindItem PlayerParty CurrentSelected)))
    (return _output)
    (else
      (bind _output_2 (CallFunction|LoopArraywithWrap PlayerParty true (Utilities|Array|FindItem EnemyParty CurrentSelected)))
      (return _output_2))))

(fn LoopArraywithWrap
  (params (Array :type Array%20of%20Actor%20Object%20References) (Countdown :type Boolean) (StartIndex :type Integer))
  (bind _returnvalue (Utilities|Array|Length Array))
  (bind _output_get (LocalVariables|SetStartingIndex (+ StartIndex _returnvalue)))
  (LocalVariables|SetGoalIndex (+ _output_get (* _returnvalue (Math|Integer|SelectInt -1 1 Countdown))))
  (bind _output_get_2 (LocalVariables|SetCurrentIndex (LocalVariables|GetStartingIndex)))
  (bind _canselect (CallFunction|CanSelect (Utilities|Array|Get(acopy) Array (Math|Integer|%(Integer) _output_get_2 _returnvalue)) :!label _label))
  (if _canselect
    (return (Utilities|Array|Get(acopy) Array (Math|Integer|%(Integer) _output_get_2 _returnvalue)))
    (else
      (if Countdown
        (Math|Integer|DecrementInt (LocalVariables|GetCurrentIndex)
          (:%20%20
            _))
        (else
          (Math|Integer|IncrementInt (LocalVariables|GetCurrentIndex)
            (:%20%20
              _))))
      (if (select Countdown (< (LocalVariables|GetGoalIndex) (LocalVariables|GetCurrentIndex)) (> (LocalVariables|GetCurrentIndex) (LocalVariables|GetGoalIndex)))
        (return 0)
        (else
          (goto _label))))))

(fn CanSelect
  (params (Actor :type Actor%20Object%20Reference))
  (return true))

(fn UpdateSelectedTarget
  (params (PlayerParty :type Array%20of%20Actor%20Object%20References) (EnemyParty :type Array%20of%20Actor%20Object%20References) (CurrentSelected :type Actor%20Object%20Reference))
  (bind _returnvalue (Utilities|Array|FindItem EnemyParty CurrentSelected))
  (bind _returnvalue_2 (Utilities|Array|FindItem PlayerParty CurrentSelected))
  (bind _returnvalue_3 (- _returnvalue 1))
  (bind _returnvalue_4 (- _returnvalue_2 1))
  (bind _canselect (CallFunction|CanSelect CurrentSelected))
  (if _canselect
    (return CurrentSelected)
    (elif (Utilities|Array|ContainsItem PlayerParty CurrentSelected)
      (bind _output (CallFunction|LoopArraywithWrap PlayerParty true _returnvalue_4))
      (Utilities|IsValid _output
        (:Is%20Valid
          (return 0))
        (:Is%20Not%20Valid
          (bind _output_2 (CallFunction|LoopArraywithWrap EnemyParty true _returnvalue_4))
          (return _output_2)))
      (else
        (bind _output_3 (CallFunction|LoopArraywithWrap EnemyParty true _returnvalue_3))
        (Utilities|IsValid _output_3
          (:Is%20Valid
            (return _output_3))
          (:Is%20Not%20Valid
            (bind _output_4 (CallFunction|LoopArraywithWrap PlayerParty true _returnvalue_3))
            (return _output_4)))))))