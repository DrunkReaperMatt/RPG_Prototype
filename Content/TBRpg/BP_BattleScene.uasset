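; Turn-based RPG battle scene, possessed by the player controller, that stages and runs fights between the active party and spawned enemies.
; StartBattle moves the party into place, then async-loads and spawns an enemy layout picked by weighted random from a data table.
; Combatants act in descending Speed order, rebuilt each round, with each component's TurnEnded event advancing the turn.
; Debug keys delegate target selection and activation to the active character's current ability.
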(event Custom|StartBattle
  (params (ReturnCharacter :type Pawn%20Object%20Reference))
  (bind _output_get (Variables|Default|SetReturnCharacter ReturnCharacter))
  (Rendering|SetActorHiddenInGame _output_get false)
  (CallFunction|MovePartytoBattle)
  (CallFunction|SpawnEnemies)
  (Pawn|Possess (Game|GetPlayerController 0) self))

(event Custom|MovePartyToBattle
  (bind _astbrpg_player_controller (Utilities|Casting|CastToTBRPG_PlayerController (Game|GetPlayerController 0))
    (:then
      (bind _output_get (Variables|Default|SetPlayer%20Controller _astbrpg_player_controller))
      (for _array_element (Variables|/Game/TBRpg/TBRPG_PlayerController.TBRPG_PlayerController_C|GetActiveParty _output_get)
        (Transformation|SetActorTransform _array_element (Transformation|GetWorldTransform (Utilities|Array|Get(acopy) (Utilities|Array|MakeArray (Variables|Default|GetPlayer2) (Variables|Default|GetPlayer3) (Variables|Default|GetPlayer1)))) false true)
        (Rendering|SetActorHiddenInGame _array_element false)))
    (:CastFailed
      (Development|PrintString "Failed to cast to TBRPG PlayerController" true true "(R=1.000000,G=0.008721,B=0.009648,A=1.000000)"))))

(event Custom|SpawnEnemies
  (bind _out_row (CallFunction|PickEnemyLayout))
  (Utilities|AsyncLoadClassAsset (.enemyclass1 _out_row)
    (:Completed
      (Utilities|Casting|CastToActorClass "/Game/TBRpg/Characters/Enemies/BP_TBEnemy.BP_TBEnemy_C")
      (bind _returnvalue (Game|SpawnActorfromClass "/Game/TBRpg/Characters/Enemies/BP_TBEnemy.BP_TBEnemy_C" (Transformation|GetWorldTransform (Variables|Default|GetEnemy1)) "Undefined" "MultiplyWithRoot" 0 0))
      (Utilities|Array|AddUnique (Variables|Default|GetEnemyParty) _returnvalue)
      (CallFunction|SetNewPartyMemberTarget 1 _returnvalue)
      (Utilities|AsyncLoadClassAsset (.enemyclass2 _out_row)
        (:Completed
          (bind _asactor (Utilities|Casting|CastToActorClass "/Game/TBRpg/Characters/Enemies/BP_TBEnemy.BP_TBEnemy_C")
            (:then
              (bind _returnvalue_2 (Game|SpawnActorfromClass _asactor (Transformation|GetWorldTransform (Variables|Default|GetEnemy2)) "Undefined" "MultiplyWithRoot" 0 0))
              (Utilities|Array|AddUnique (Variables|Default|GetEnemyParty) _returnvalue_2)
              (CallFunction|SetNewPartyMemberTarget 2 _returnvalue_2)
              (Utilities|AsyncLoadClassAsset (.enemyclass3 _out_row)
                (:Completed
                  _)))
            (:CastFailed
              _))
          (bind _asactor_2 (Utilities|Casting|CastToActorClass "/Game/TBRpg/Characters/Enemies/BP_TBEnemy.BP_TBEnemy_C")
            (:then
              (bind _returnvalue_3 (Game|SpawnActorfromClass _asactor_2 (Transformation|GetWorldTransform (Variables|Default|GetEnemy3)) "Undefined" "MultiplyWithRoot" 0 0))
              (Utilities|Array|AddUnique (Variables|Default|GetEnemyParty) _returnvalue_3)
              (CallFunction|SetNewPartyMemberTarget 3 _returnvalue_3))
            (:CastFailed
              _))
          (CallFunction|SetTurnOrder)
          (CallFunction|NextCharacter))))))

(event Custom|NextCharacter
  (bind _player_controller (Variables|Default|GetPlayer%20Controller))
  (bind _player_controller_2 (Variables|Default|GetPlayer%20Controller))
  (bind _turnorderactors (Variables|Default|GetTurnOrderActors))
  (bind _activeparty (Variables|/Game/TBRpg/TBRPG_PlayerController.TBRPG_PlayerController_C|GetActiveParty _player_controller))
  (bind _activeparty_2 (Variables|/Game/TBRpg/TBRPG_PlayerController.TBRPG_PlayerController_C|GetActiveParty _player_controller_2))
  (if (>= (Variables|Default|GetTurnOrderIndex) (Utilities|Array|Length _turnorderactors))
    (Variables|Default|SetTurnOrderIndex 0)
    (CallFunction|SetTurnOrder)
    (CallFunction|NextCharacter)
    (else
      (bind _component (Class|BPITurnBasedCombat|GetTurnBasedComponent(Message) (Utilities|Array|Get(acopy) _turnorderactors (Variables|Default|GetTurnOrderIndex))))
      (bind _currentvaluewithmod (Default|GetAttributeCurrent _component "HP"))
      (if (> _currentvaluewithmod 0.0)
        (Class|BPITurnBasedCombat|SetTurnActive(Message) (Variables|Default|GetActiveActor) false)
        (bind _output_get (Variables|Default|SetActiveActor (Utilities|Array|Get(acopy) _turnorderactors (Variables|Default|GetTurnOrderIndex))))
        (Class|BPITurnBasedCombat|SetTurnActive(Message) _output_get true)
        (Math|Integer|IncrementInt (Variables|Default|GetTurnOrderIndex)
          (:%20%20
            (bind _component_2 (Class|BPITurnBasedCombat|GetTurnBasedComponent(Message) (Variables|Default|GetActiveActor)))
            (EventDispatchers|BindEventtoTurnEnded _component_2 (delegate Custom|TurnEnded_Event))
            (Default|StartTurn _component_2)
            (Variables|Default|SetIsPlayerTurn (Utilities|Array|ContainsItem (Variables|/Game/TBRpg/TBRPG_PlayerController.TBRPG_PlayerController_C|GetActiveParty (Variables|Default|GetPlayer%20Controller)) (Variables|Default|GetActiveActor)))
            (bind _component_3 (Class|BPITurnBasedCombat|GetTurnBasedComponent(Message) (Variables|Default|GetActiveActor)))
            (CallFunction|SetSelectionbyIndex (Math|Integer|SelectInt (Utilities|Array|FindItem _activeparty (Variables|/Game/TBRpg/Components/AbilitySystemComponent.AbilitySystemComponent_C|GetTarget _component_3)) (Utilities|Array|FindItem (Variables|Default|GetEnemyParty) (Variables|/Game/TBRpg/Components/AbilitySystemComponent.AbilitySystemComponent_C|GetTarget _component_3)) (Utilities|Array|ContainsItem _activeparty (Variables|/Game/TBRpg/Components/AbilitySystemComponent.AbilitySystemComponent_C|GetTarget _component_3))))
            (bind _output_get_2 (Variables|Default|SetCurrentAbility (Utilities|Array|Get(acopy) (Variables|/Game/TBRpg/Components/AbilitySystemComponent.AbilitySystemComponent_C|GetActiveAbilities _component_3))))
            (Default|UpdateSelectedTarget _output_get_2 (Variables|/Game/TBRpg/TBRPG_PlayerController.TBRPG_PlayerController_C|GetActiveParty (Variables|Default|GetPlayer%20Controller)) (Variables|Default|GetEnemyParty) (Variables|Default|GetTargetedActor))
            (bind _output_get_3 (Variables|Default|SetOwnPartySelected (Utilities|Array|ContainsItem _activeparty_2 (Variables|/Game/TBRpg/Components/AbilitySystemComponent.AbilitySystemComponent_C|GetTarget _component_2))))
            (CallFunction|SetSelectionbyIndex (Math|Integer|SelectInt (Utilities|Array|FindItem _activeparty_2 (Variables|/Game/TBRpg/Components/AbilitySystemComponent.AbilitySystemComponent_C|GetTarget _component_2)) (Utilities|Array|FindItem (Variables|Default|GetEnemyParty) (Variables|/Game/TBRpg/Components/AbilitySystemComponent.AbilitySystemComponent_C|GetTarget _component_2)) _output_get_3))))
        (else
          (Math|Integer|IncrementInt (Variables|Default|GetTurnOrderIndex)))))))

(event Custom|TurnEnded_Event
  (Utilities|FlowControl|DelayUntilNextTick)
  (CallFunction|NextCharacter))

(event Input|KeyboardEvents|DebugKeyW
  (params (Key :type Key%20Structure :default "None") (ActionValue :type Input%20Action%20Value%20Structure))
  (:Pressed
    (if (Variables|Default|GetIsPlayerTurn)
      (bind _currentability (Variables|Default|GetCurrentAbility)
        (:then
          (bind _output (Default|SelectUp _currentability (Variables|/Game/TBRpg/TBRPG_PlayerController.TBRPG_PlayerController_C|GetActiveParty (Variables|Default|GetPlayer%20Controller)) (Variables|Default|GetEnemyParty) (Variables|Default|GetTargetedActor)))
          (CallFunction|SetNewSelectedTarget _output))
        (:else)))))

(event Input|KeyboardEvents|DebugKeyA
  (params (Key :type Key%20Structure :default "None") (ActionValue :type Input%20Action%20Value%20Structure))
  (:Pressed
    (if (Variables|Default|GetIsPlayerTurn)
      (bind _currentability (Variables|Default|GetCurrentAbility)
        (:then
          (bind _output (Default|SelectOtherParty (stale Input|KeyboardEvents|DebugKeyD _currentability) (Variables|/Game/TBRpg/TBRPG_PlayerController.TBRPG_PlayerController_C|GetActiveParty (Variables|Default|GetPlayer%20Controller)) (Variables|Default|GetEnemyParty) (Variables|Default|GetTargetedActor)))
          (CallFunction|SetNewSelectedTarget _output))
        (:else)))))

(event Input|KeyboardEvents|DebugKeyS
  (params (Key :type Key%20Structure :default "None") (ActionValue :type Input%20Action%20Value%20Structure))
  (:Pressed
    (if (Variables|Default|GetIsPlayerTurn)
      (bind _currentability (Variables|Default|GetCurrentAbility)
        (:then
          (bind _output (Default|SelectDown _currentability (Variables|/Game/TBRpg/TBRPG_PlayerController.TBRPG_PlayerController_C|GetActiveParty (Variables|Default|GetPlayer%20Controller)) (Variables|Default|GetEnemyParty) (Variables|Default|GetTargetedActor)))
          (CallFunction|SetNewSelectedTarget _output))
        (:else)))))

(event Input|KeyboardEvents|DebugKeyD
  (params (Key :type Key%20Structure :default "None") (ActionValue :type Input%20Action%20Value%20Structure))
  (:Pressed
    (if (Variables|Default|GetIsPlayerTurn)
      (bind _currentability (Variables|Default|GetCurrentAbility)
        (:then
          (bind _output (Default|SelectOtherParty _currentability (Variables|/Game/TBRpg/TBRPG_PlayerController.TBRPG_PlayerController_C|GetActiveParty (Variables|Default|GetPlayer%20Controller)) (Variables|Default|GetEnemyParty) (Variables|Default|GetTargetedActor)))
          (CallFunction|SetNewSelectedTarget _output))
        (:else)))))

(event Input|KeyboardEvents|DebugKeyEnter
  (params (Key :type Key%20Structure :default "None") (ActionValue :type Input%20Action%20Value%20Structure))
  (:Pressed
    (if true
      (bind _currentability (Variables|Default|GetCurrentAbility)
        (:then
          (Default|ActivateAbility _currentability))
        (:else)))))

(fn ConstructionScript)

(fn GetBattleCharacters
  (LocalVariables|SetOutputArray (Variables|/Game/TBRpg/TBRPG_PlayerController.TBRPG_PlayerController_C|GetActiveParty (Variables|Default|GetPlayer%20Controller)))
  (for _array_element (Variables|Default|GetEnemyParty)
    (Utilities|Array|AddUnique (LocalVariables|GetOutputArray) _array_element))
  (return (LocalVariables|GetOutputArray)))

(fn PickEnemyLayout
  (bind _encounterrate (Variables|Default|GetEncounterRate))
  (if (== (Class|DataTableFunctionLibrary|GetDataTableRowStruct _encounterrate) "/Game/TBRpg/DataAssets/BasicEncounterTAble.BasicEncounterTAble")
    (bind _outrownames (DataTable|GetDataTableRowNames _encounterrate))
    (for _array_element _outrownames
      (bind _returnvalue (Utilities|GetDataTableRow "/Game/TBRpg/DataAssets/BasicEncounterTAble.BasicEncounterTAble" _array_element)
        (:then
          (LocalVariables|SetTotalWeight (+ (LocalVariables|GetTotalWeight) (.Weight (Utilities|Struct|BreakEnemyEncounter _returnvalue)))))))
    (LocalVariables|SetTargetWeight (Math|Random|RandomFloatinRange 0.0 (LocalVariables|GetTotalWeight)))
    (bind _outrownames_2 (DataTable|GetDataTableRowNames "/Game/TBRpg/DataAssets/BasicEncounterTAble.BasicEncounterTAble"))
    (for _array_element_2 _outrownames_2
      (bind _returnvalue_2 (Utilities|GetDataTableRow "/Game/TBRpg/DataAssets/BasicEncounterTAble.BasicEncounterTAble" _array_element_2)
        (:then
          (bind _output_get (LocalVariables|SetCOuntUpWeight (+ (LocalVariables|GetCOuntUpWeight) (.Weight (Utilities|Struct|BreakEnemyEncounter _returnvalue_2)))))
          (if (<= (LocalVariables|GetTargetWeight) _output_get)
            (return _returnvalue_2)))))
    (else
      (return ""))))

(fn SetTurnOrder
  (for _array_element (CallFunction|GetBattleCharacters)
    (bind _component (Class|BPITurnBasedCombat|GetTurnBasedComponent(Message) _array_element))
    (bind _currentvaluewithmod (Default|GetAttributeCurrent _component "Speed"))
    (Utilities|Array|Add (LocalVariables|GetSpeeds) _currentvaluewithmod))
  (Class|KismetArrayLibrary|SortFloatArray (LocalVariables|GetSpeeds) false "Descending")
  (for _array_element_2 (LocalVariables|GetSpeeds)
    (for _array_element_3 (CallFunction|GetBattleCharacters)
      (bind _component_2 (Class|BPITurnBasedCombat|GetTurnBasedComponent(Message) _array_element_3))
      (bind _currentvaluewithmod_2 (Default|GetAttributeCurrent _component_2 "Speed"))
      (if (== _array_element_2 _currentvaluewithmod_2)
        (Utilities|Array|AddUnique (LocalVariables|GetTurnOrder) _array_element_3))))
  (Variables|Default|SetTurnOrderActors (LocalVariables|GetTurnOrder)))

(fn SetSelectionbyIndex
  (params (Index :type Integer))
  (if (Variables|Default|GetOwnPartySelected)
    (CallFunction|SetSelectioninArray Index (Variables|/Game/TBRpg/TBRPG_PlayerController.TBRPG_PlayerController_C|GetActiveParty (Variables|Default|GetPlayer%20Controller)))
    (else
      (CallFunction|SetSelectioninArray Index (Variables|Default|GetEnemyParty)))))

(fn SetSelectioninArray
  (params (Index :type Integer) (Array :type Array%20of%20Actor%20Object%20References))
  (bind _returnvalue (Utilities|Array|LastIndex Array))
  (if (> Index _returnvalue)
    (Variables|Default|SetSelectionIndex 0)
    (elif (< Index 0)
      (Variables|Default|SetSelectionIndex _returnvalue)
      (else
        (Variables|Default|SetSelectionIndex Index))))
  (Variables|Default|SetTargetedActor (Utilities|Array|Get(acopy) Array (Variables|Default|GetSelectionIndex))))

(fn SetNewSelectedTarget
  (params (Actor :type Actor%20Object%20Reference))
  (Utilities|IsValid Actor
    (:Is%20Valid
      (Class|BPITurnBasedCombat|SetTargeted(Message) Actor true)
      (Class|BPITurnBasedCombat|SetTargeted(Message) (Variables|Default|GetTargetedActor) false)
      (bind _output_get (Variables|Default|SetTargetedActor Actor))
      (CallFunction|SetNewPartyMemberTarget (Utilities|Array|FindItem (Variables|/Game/TBRpg/TBRPG_PlayerController.TBRPG_PlayerController_C|GetActiveParty (Variables|Default|GetPlayer%20Controller)) (Variables|Default|GetActiveActor)) _output_get))))

(fn SetNewPartyMemberTarget
  (params (PartyMemberIndex :type Integer) (Target :type Actor%20Object%20Reference))
  (bind _component (Class|BPITurnBasedCombat|GetTurnBasedComponent(Message) (Utilities|Array|Get(acopy) (Variables|/Game/TBRpg/TBRPG_PlayerController.TBRPG_PlayerController_C|GetActiveParty (Variables|Default|GetPlayer%20Controller)) PartyMemberIndex)))
  (Variables|/Game/TBRpg/Components/AbilitySystemComponent.AbilitySystemComponent_C|SetTarget _component Target))