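; Base actor for turn-based RPG characters, built around an ability system component that it exposes through GetTurnBasedComponent.
; On BeginPlay it applies a small random Speed effect to itself.
; Turn start activates GA_Wait and shows a turn outline through the skeletal mesh overlay material.
; Targeting swaps in a selection outline, then restores the turn outline or clears the overlay, depending on whose turn it is.
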(event EventBeginPlay
  (Default|ApplyEffecttoSelf (Variables|Default|GetAbilitySystemComponent) "Speed" (Math|Random|RandomFloatinRange -2.0 2.0) "NewEnumerator0" "NewEnumerator4" "NewEnumerator0"))

(event Collision|EventActorBeginOverlap
  (params (OtherActor :type Actor%20Object%20Reference)))

(event EventTick
  (params (DeltaSeconds :type Float%20%28single-precision%29)))

(event EventSetTurnActive
  (params (IsActive :type Boolean))
  (if IsActive
    (Default|ActivateSingleAbility (Variables|Default|GetAbilitySystemComponent) "/Game/TBRpg/GameplayAbilities/GA_Wait.GA_Wait_C" 0 false)
    (Rendering|Material|SetOverlayMaterial (Variables|Default|GetSkeletalMesh) "/Game/TBRpg/Characters/TurnOutline.TurnOutline" :!class /Script/Engine.MeshComponent)
    (else
      (Rendering|Material|SetOverlayMaterial (Variables|Default|GetSkeletalMesh) 0 :!class /Script/Engine.MeshComponent))))

(event EventSetTargeted
  (params (IsTargeted :type Boolean))
  (if IsTargeted
    (Rendering|Material|SetOverlayMaterial (Variables|Default|GetSkeletalMesh) "/Game/TBRpg/Characters/SelectionOutline.SelectionOutline" :!class /Script/Engine.MeshComponent)
    (elif (Variables|/Game/TBRpg/Components/AbilitySystemComponent.AbilitySystemComponent_C|GetIsTurn (Variables|Default|GetAbilitySystemComponent))
      (Rendering|Material|SetOverlayMaterial (Variables|Default|GetSkeletalMesh) "/Game/TBRpg/Characters/TurnOutline.TurnOutline" :!class /Script/Engine.MeshComponent)
      (else
        (Rendering|Material|SetOverlayMaterial (Variables|Default|GetSkeletalMesh) 0 :!class /Script/Engine.MeshComponent)))))

(fn ConstructionScript)

(fn GetTurnBasedComponent
  (return (Variables|Default|GetAbilitySystemComponent)))