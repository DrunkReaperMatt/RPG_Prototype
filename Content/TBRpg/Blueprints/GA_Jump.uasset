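; GA_Jump is a gameplay ability that makes the owning Character jump.
; On activation it commits the ability, calls Jump and binds to the Character's movement mode changed delegate.
; The ability stays active until a mode change returns the Character to Walking, and ends at once if the commit or Character cast fails.
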(event Custom|CustomEvent
  (params (Character :type Character%20Object%20Reference) (PrevMovementMode :type EMovementMode%20Enum :default "MOVE_None") (PreviousCustomMode :type Byte))
  (if (Utilities|Enum|Equal(Enum) (Variables|/Script/Engine.CharacterMovementComponent|GetMovementMode (Variables|/Script/Engine.Character|GetCharacterMovement (stale EventActivateAbility _ascharacter))) "MOVE_Walking")
    (CallFunction|EndAbility)))

(event EventActivateAbility
  (bind _commited (CallFunction|CommitAbility))
  (if _commited
    (bind _ascharacter (Utilities|Casting|CastToCharacter (Components|GetOwner))
      (:then
        (Character|Jump _ascharacter)
        (Character|BindEventtoMovementModeChangedDelegate _ascharacter (delegate Custom|CustomEvent)))
      (:CastFailed
        (CallFunction|EndAbility :!label _label)))
    (else
      (goto _label))))

(fn ConstructionScript
  (|CallParentFunction))