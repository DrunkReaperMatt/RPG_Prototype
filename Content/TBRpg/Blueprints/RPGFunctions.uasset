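; RPGFunctions holds CanDoAbility, a helper that reports whether an ability system can afford an ability's attribute cost.
; It reads the cost name and amount from the class defaults, then compares the matching attribute's current value against that amount.
; The loop returns false at the first non-matching attribute, so only the first entry is effectively checked, and an empty list also returns false.
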(fn CanDoAbility
  (params (OwningAbilitySystem :type Ability%20System%20Component%20Object%20Reference) (AttributeClass :type BP%20Turn%20Based%20Ability%20Class%20Reference))
  (bind _cost (Utilities|GetClassDefaults AttributeClass))
  (bind (_cost_2 _name) (Utilities|Struct|BreakAttributeCost _cost))
  (bind _output_get (LocalVariables|SetAbilitySystem OwningAbilitySystem))
  (for _array_element (Variables|/Game/TBRpg/Blueprints/AbilitySystemComponent.AbilitySystemComponent_C|GetAttributes _output_get)
    (if (== (.name _array_element) _name)
      (bind _currentvaluewithmod (Default|GetAttributeCurrent (LocalVariables|GetAbilitySystem) _name))
      (return (>= _currentvaluewithmod _cost_2))
      (else
        (return false))))
  (return false))