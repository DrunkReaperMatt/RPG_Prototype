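; Ability system component for a turn-based RPG that reads named attributes and applies effects to them.
; Getters search Attributes by name and return min, max or current value plus its modifier.
; ApplyEffectToTarget, also wrapped for self, constructs and applies a BP_TurnEffect, relaying its update event through AttributeUpdated.
; Only Infinite and Temporary effects enter ActiveEffects, stored on the applying component rather than the target.
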(event EventBeginPlay)

(event EventTick
  (params (DeltaSeconds :type Float%20%28single-precision%29)))

(fn GetAttributeMin
  (params (Name :type Name))
  (for _array_element (Variables|Default|GetAttributes)
    (if (== (.name _array_element) Name)
      (return (+ (.MinValue (Utilities|Struct|BreakStat (.stat _array_element))) (.MinValueMod (Utilities|Struct|BreakStat (.stat _array_element))))))))

(fn GetAttributeMax
  (params (Name :type Name))
  (for _array_element (Variables|Default|GetAttributes)
    (if (== (.name _array_element) Name)
      (return (+ (.MaxValue (Utilities|Struct|BreakStat (.stat _array_element))) (.MaxValueMod (Utilities|Struct|BreakStat (.stat _array_element))))))))

(fn GetAttributeCurrent
  (params (Name :type Name))
  (for _array_element (Variables|Default|GetAttributes)
    (if (== (.name _array_element) Name)
      (return (+ (.CurrentValue (Utilities|Struct|BreakStat (.stat _array_element))) (.CurrentValueMod (Utilities|Struct|BreakStat (.stat _array_element))))))))

(fn ApplyEffecttoTarget
  (params (TargetComponent :type Ability%20System%20Component%20Object%20Reference) (AttributeToEffect :type Name) (Magnitude :type Float%20%28double-precision%29) (EffectType :type EffectType%20Enum :default "NewEnumerator0") (TargetStat :type TargetStat%20Enum :default "NewEnumerator0") (EffectMath :type EffectMath%20Enum :default "NewEnumerator0") (EffectTurnCounter :type Integer))
  (bind _returnvalue (Game|ConstructObjectfromClass TargetComponent "/Game/TBRpg/Blueprints/BP_TurnEffect.BP_TurnEffect_C" EffectType TargetComponent AttributeToEffect TargetStat EffectMath Magnitude EffectTurnCounter))
  (EventDispatchers|BindEventtoUpdateAttribute _returnvalue (EventDispatchers|CreateEvent TargetComponent :!event OnAttributeUpdated))
  (switch Utilities|FlowControl|Switch|SwitchonEffectType EffectType
    (:NewEnumerator0
      _)
    (:NewEnumerator1
      _)
    (:NewEnumerator2
      (Utilities|Array|AddUnique (Variables|Default|GetActiveEffects) _returnvalue :!label _label))
    (:NewEnumerator3
      (goto _label)))
  (Default|ApplyEffect _returnvalue)
  (return _returnvalue))

(fn OnAttributeUpdated
  (params (Attribute :type Attribute%20Structure))
  (Default|CallAttributeUpdated Attribute))

(fn ApplyEffecttoSelf
  (params (AttributeToEffect :type Name) (Magnitude :type Float%20%28double-precision%29) (EffectType :type EffectType%20Enum :default "NewEnumerator0") (TargetStat :type TargetStat%20Enum :default "NewEnumerator0") (EffectMath :type EffectMath%20Enum :default "NewEnumerator0") (EffectTurnCounter :type Integer))
  (CallFunction|ApplyEffecttoTarget self AttributeToEffect Magnitude EffectType TargetStat EffectMath EffectTurnCounter))