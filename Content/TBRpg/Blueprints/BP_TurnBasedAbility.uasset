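; BP_TurnBasedAbility is an actor-based ability for the turn-based RPG, with an empty ActivateAbility event.
; CommitAbility checks CanDoAbility against the owning ability component and its own class, then applies the negated cost to the cost attribute as a self effect.
; A failed commit destroys the actor and returns false.
; EndAbility fires the AbilityEnd dispatcher, then destroys the actor, so neither path leaves the instance alive.
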(event Custom|ActivateAbility)

(event Custom|EndAbility
  (Default|CallAbilityEnd self)
  (Actor|DestroyActor))

(fn ConstructionScript)

(fn CommitAbility
  (bind _cost (Variables|Default|GetCost))
  (bind _cando (CallFunction|CanDoAbility (Variables|Default|GetOwningAbilityComponent) (Utilities|GetClass self)))
  (if _cando
    (Default|ApplyEffecttoSelf (Variables|Default|GetOwningAbilityComponent) (.name _cost) (* (.cost _cost) -1.0) "NewEnumerator0" "NewEnumerator4" "NewEnumerator0")
    (return true)
    (else
      (Actor|DestroyActor)
      (return false))))