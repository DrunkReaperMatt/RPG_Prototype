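; BP_EquipmentMesh is a static mesh component that represents one equipment slot on its owning actor in the turn-based RPG.
; Equip ignores items for other slots, otherwise it unequips first, stores the item and displays its mesh.
; Each item modifier becomes an effect on the owner through its turn-based component interface, tracked in an Effects list.
; Unequip ends those tracked effects, clears the list and removes the mesh.
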(event Custom|Equip
  (params (Equipment :type Equipment%20Data%20Asset%20Object%20Reference))
  (if (== (Variables|/Game/TBRpg/Blueprints/DataAssets/EquipmentDataAsset.EquipmentDataAsset_C|GetSlotName Equipment) (Variables|Default|GetSlotName))
    (CallFunction|Unequip)
    (Variables|Default|SetCurrently%20Equiped Equipment)
    (bind _component (Class|BPITurnBasedCombat|GetTurnBasedComponent(Message) (Components|GetOwner)))
    (for _array_element (Variables|/Game/TBRpg/Blueprints/DataAssets/EquipmentDataAsset.EquipmentDataAsset_C|GetModifiers (Variables|Default|GetCurrently%20Equiped))
      (bind _effect_ref (Default|ApplyEffecttoSelf _component (.name _array_element) (.magnitude _array_element) "NewEnumerator3" (.statvalue _array_element) (.operation _array_element)))
      (Utilities|Array|AddUnique (Variables|Default|GetEffects) _effect_ref))
    (Components|StaticMesh|SetStaticMesh (Variables|/Game/TBRpg/Blueprints/DataAssets/EquipmentDataAsset.EquipmentDataAsset_C|GetMesh (Variables|Default|GetCurrently%20Equiped)))))

(event Custom|Unequip
  (bind _effects (Variables|Default|GetEffects))
  (for _array_element _effects
    (Default|EndEffect _array_element))
  (Utilities|Array|Clear _effects)
  (Components|StaticMesh|SetStaticMesh 0))